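; Default pawn Blueprint that supplies an aim mode and query functions for attack range, interaction distance and bone positions.
; It caches the camera's field of view on BeginPlay, and ToggleAimMode switches between that base value and the aim FOV while storing the aiming state.
; That state makes GetAttackRange return shoot range when aiming and melee range otherwise.
; GetBoneLocation reads bone positions from the skeletal mesh in a given transform space.
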(event `self.ReceiveBeginPlay`
  (bind _camera (`self.Camera`))
  (`/Engine/EditorBlueprintResources/StandardMacros.IsValid` _camera
    (:`Is Valid`
      (set `self.BaseFOV` (`CameraComponent.FieldOfView` _camera)))))

(fn `GetAttackRange`
  (returns (AttackRange :type "Float (double-precision)"))
  (if (`self.IsAiming`)
    (return (`self.ShootRange`))
    (else
      (return (`self.MeleeRange`)))))

(fn `GetBoneLocation`
  (params (BoneName :type Name) (TransformSpace :type "ERelativeTransformSpace Enum" :default "RTS_World"))
  (returns (Location :type "Vector Structure"))
  (locals (NewLocalVar :type "ERelativeTransformSpace Enum" :default "RTS_World"))
  (bind _skeletalmesh (`self.SkeletalMesh`))
  (bind _returnvalue_location (`KismetMathLibrary.BreakTransform` (`SkinnedMeshComponent.GetBoneTransform` _skeletalmesh BoneName TransformSpace)))
  (`/Engine/EditorBlueprintResources/StandardMacros.IsValid` _skeletalmesh
    (:`Is Valid`
      (return _returnvalue_location))))

(fn `GetInteractDistance`
  (returns (InteractDistance :type "Float (double-precision)"))
  (return (`self.InteractDistance`)))

(fn `ToggleAimMode`
  (params (IsAiming :type Boolean))
  (locals (newFOV :type "Float (double-precision)"))
  (bind _camera (`self.Camera`))
  (if IsAiming
    (`CameraComponent.SetFieldOfView` _camera (`self.AimFOV`))
    (else
      (`CameraComponent.SetFieldOfView` _camera (`self.BaseFOV`))))
  (set `self.IsAiming` IsAiming)
  (return))

(fn `UserConstructionScript`)