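; BP_Citizen is an environment Blueprint for a citizen object that reacts to interaction and damage.
; Interact calls SetRandomColor, which writes a random RGB value into the Color parameter on the static mesh's materials.
; TakeDamage applies a velocity-change impulse to the capsule, using DamageImpulseForce on the Z axis, so the citizen gets knocked vertically.
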(event `/Game/A4GPContent/Datas/Interfaces/I_Interactable.Interact`
  (`self.SetRandomColor`))

(event `/Game/A4GPContent/Datas/Interfaces/I_Damageable.Take Damage`
  (bind _capsule (`self.Capsule`))
  (`/Engine/EditorBlueprintResources/StandardMacros.IsValid` _capsule
    (:`Is Valid`
      (`PrimitiveComponent.AddImpulse` _capsule (`KismetMathLibrary.MakeVector` 0.0 0.0 (`self.DamageImpulseForce`)) "None" true))))

(fn `SetRandomColor`
  (bind _staticmesh (`self.StaticMesh`))
  (`/Engine/EditorBlueprintResources/StandardMacros.IsValid` _staticmesh
    (:`Is Valid`
      (`MeshComponent.SetVectorParameterValueOnMaterials` _staticmesh "Color" (`KismetMathLibrary.MakeVector` (`KismetMathLibrary.RandomFloatInRange` 0.0 1.0) (`KismetMathLibrary.RandomFloatInRange` 0.0 1.0) (`KismetMathLibrary.RandomFloatInRange` 0.0 1.0))))))

(fn `UserConstructionScript`)