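; BP_RandomLight is an environment light Blueprint whose four point lights share one random color and can be switched on or off together.
; On BeginPlay it gathers the lights, applies a color with each channel randomized within a mid range, then switches them off.
; SwitchLights toggles intensity between LightIntensity and zero rather than changing visibility.
; A setter is provided for a random-lights manager reference, which is not otherwise used here.
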(event `self.ReceiveBeginPlay`
  (set `self.Lights` (`|MakeArray` (`self.PointLight0`) (`self.PointLight1`) (`self.PointLight2`) (`self.PointLight3`)))
  (`self.ChooseRandomLightColor`)
  (`self.SwitchLights` false))

(fn `ChooseRandomLightColor`
  (locals (Color :type "Vector Structure"))
  (bind _output_get (set `local.Color` (`KismetMathLibrary.MakeVector` (`KismetMathLibrary.RandomFloatInRange` 0.2 0.8) (`KismetMathLibrary.RandomFloatInRange` 0.2 0.8) (`KismetMathLibrary.RandomFloatInRange` 0.2 0.8))))
  (for _array_element (`self.Lights`)
    (`/Engine/EditorBlueprintResources/StandardMacros.IsValid` _array_element
      (:`Is Valid`
        (`LightComponent.SetLightColor` _array_element (`KismetMathLibrary.Conv_VectorToLinearColor` _output_get) true)))))

(fn `SetRandomLightsManager`
  (params (Manager :type "/Game/A4GPContent/BP/Environment/BP_RandomLightsManager Object Reference"))
  (set `self.Manager` Manager))

(fn `SwitchLights`
  (params (IsOn :type Boolean))
  (for _array_element (`self.Lights`)
    (`/Engine/EditorBlueprintResources/StandardMacros.IsValid` _array_element
      (:`Is Valid`
        (if IsOn
          (`LightComponent.SetIntensity` _array_element (`self.LightIntensity`))
          (else
            (`LightComponent.SetIntensity` _array_element 0.0)))))))

(fn `UserConstructionScript`)