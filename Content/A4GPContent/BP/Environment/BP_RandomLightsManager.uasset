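; BP_RandomLightsManager spawns a random number of BPRandomLight actors and lights them in random batches whenever its linked Button is pressed.
; At BeginPlay it spaces the lights along world X with random yaw, registers itself on each and binds the button.
; Each press switches on and removes a random subset of UnlitLights, or all when five or fewer remain.
; A press with none unlit switches everything off and refills the pool.
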(event `self.ReceiveBeginPlay`
  (bind _button (`self.Button`))
  (`self.SpawnLights`)
  (`/Engine/EditorBlueprintResources/StandardMacros.IsValid` _button
    (:`Is Valid`
      (add `/Game/A4GPContent/BP/Environment/BP_Button.OnPressed` _button (delegate `ButtonPressed`)))))

(event `ButtonPressed`
  (bind _unlitlights (`self.UnlitLights`))
  (bind _alllights (`self.AllLights`))
  (bind _unlitlights_2 (`self.UnlitLights`))
  (bind _returnvalue (`KismetArrayLibrary.Array_Length` _unlitlights))
  (`KismetSystemLibrary.PrintString` (`KismetStringLibrary.Concat_StrStr` "Unlit array length :" (`KismetStringLibrary.Conv_IntToString` _returnvalue)))
  (if (> _returnvalue 0)
    (if (<= _returnvalue 5)
      (`self.SwitchAllLightsOf` _unlitlights true true)
      (else
        (bind _randomunlitlights (`self.GetRandomUnlitLights` (`KismetMathLibrary.RandomIntegerInRange` 1 (+ _returnvalue 1))))
        (`self.SwitchAllLightsOf` _randomunlitlights true true)))
    (else
      (`self.SwitchAllLightsOf` _alllights)
      (`KismetArrayLibrary.Array_Clear` _unlitlights_2)
      (for _array_element _alllights
        (`KismetArrayLibrary.Array_Add` _unlitlights_2 _array_element)))))

(fn `GetRandomUnlitLights`
  (params (MaxNumber :type Integer))
  (returns (RandomUnlitLights :type "Array of /Game/A4GPContent/BP/Environment/BP_RandomLight Object Reference"))
  (locals (ReturnArray :type "Array of /Game/A4GPContent/BP/Environment/BP_RandomLight Object Reference") (DesiredReturnArraySize :type Integer) (RandomIndex :type Integer :default 0))
  (bind _unlitlights (`self.UnlitLights`))
  (bind _returnvalue (`KismetArrayLibrary.Array_Length` _unlitlights))
  (bind _output_get (set `local.DesiredReturnArraySize` (`KismetMathLibrary.RandomIntegerInRange` 1 (+ MaxNumber 1))))
  (while (< (`KismetArrayLibrary.Array_Length` (`local.ReturnArray`)) _output_get)
    (if (> _returnvalue 0)
      (bind _output_get_2 (set `local.RandomIndex` (`KismetMathLibrary.RandomInteger` _returnvalue)))
      (`KismetArrayLibrary.Array_Add` (`local.ReturnArray`) (`|GetArrayItem` _unlitlights _output_get_2))
      (`KismetArrayLibrary.Array_Remove` _unlitlights _output_get_2)
      (else
        (`KismetSystemLibrary.PrintString` (`KismetStringLibrary.Concat_StrStr` "Unlit Lights After Interact : " (`KismetStringLibrary.Conv_IntToString` _returnvalue)) :!label _label)
        (return (`local.ReturnArray`)))))
  (goto _label))

(fn `SpawnLights`
  (locals (NumberOfLightsToSpawn :type Integer))
  (bind _returnvalue (/ (`self.SpawnRange`) 2.0))
  (bind _output_get (set `local.NumberOfLightsToSpawn` (`KismetMathLibrary.RandomIntegerInRange` (`self.LightsToSpawn_Min`) (`self.LightsToSpawn_Max`))))
  (`KismetSystemLibrary.PrintString` (`KismetStringLibrary.Concat_StrStr` "Number of lights to spawn : " (`KismetStringLibrary.Conv_IntToString` _output_get)))
  (for _index (range 1 (+ _output_get 1))
    (bind _returnvalue_2 (`|SpawnActorFromClass` (`self.BP_RandomLight`) (`KismetMathLibrary.MakeTransform` (`KismetMathLibrary.MakeVector` (`KismetMathLibrary.Lerp` (- 0.0 _returnvalue) _returnvalue (/ (`KismetMathLibrary.Conv_IntToDouble` _index) (`KismetMathLibrary.Conv_IntToDouble` _output_get)))) (`KismetMathLibrary.MakeRotator` 0.0 0.0 (`KismetMathLibrary.RandomFloatInRange` -180.0 180.0))) "AlwaysSpawn" "MultiplyWithRoot" null null))
    (`/Game/A4GPContent/BP/Environment/BP_RandomLight.SetRandomLightsManager` _returnvalue_2 self)
    (`KismetArrayLibrary.Array_Add` (`self.AllLights`) _returnvalue_2)
    (`KismetArrayLibrary.Array_Add` (`self.UnlitLights`) _returnvalue_2)))

(fn `SwitchAllLightsOf`
  (params (LightsArray :type "Array of /Game/A4GPContent/BP/Environment/BP_RandomLight Object Reference") (IsOn :type Boolean) (DoClearArray :type Boolean))
  (for _array_element LightsArray
    (`/Engine/EditorBlueprintResources/StandardMacros.IsValid` _array_element
      (:`Is Valid`
        (`/Game/A4GPContent/BP/Environment/BP_RandomLight.SwitchLights` _array_element IsOn))))
  (if DoClearArray
    (`KismetArrayLibrary.Array_Clear` LightsArray)))

(fn `UserConstructionScript`)