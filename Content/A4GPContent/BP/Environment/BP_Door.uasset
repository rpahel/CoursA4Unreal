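; BP_Door is an environment door that toggles between open and closed when it receives an Interact event.
; It snaps the Door's relative rotation instantly between zero and a yaw set by OpeningAngle, then flips the IsOpen flag.
; If the Door reference is invalid, it prints a red on-screen error naming the actor instead.
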(event `/Game/A4GPContent/Datas/Interfaces/I_Interactable.Interact`
  (bind _door (`self.Door`))
  ;[1 1 1] Check door validity
  (if (`KismetSystemLibrary.IsValid` _door)
    ;[1 1 1] Change door rotation
    (if (`self.IsOpen`)
      (`SceneComponent.K2_SetRelativeRotation` :`self` _door)
      (else
        (`SceneComponent.K2_SetRelativeRotation` _door (`KismetMathLibrary.MakeRotator` 0.0 0.0 (`self.OpeningAngle`)) false false)))
    ;[1 1 1] Update IsOpen
    (set `self.IsOpen` (not (`self.IsOpen`)))
    (else
      (`KismetSystemLibrary.PrintString` (`KismetStringLibrary.Concat_StrStr` (`KismetSystemLibrary.GetDisplayName` self) " : Door is not valid !") true true (struct :`R` 1.0 :`A` 1.0) 10.0))))

(fn `UserConstructionScript`)