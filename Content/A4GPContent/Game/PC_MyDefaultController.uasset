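; Player controller that drives BP_MyDefaultPawn with Enhanced Input for flying-style movement, looking and interacting.
; BeginPlay adds the default mapping context and caches the pawn; Destroyed removes the context.
; Move input pushes the pawn along yaw-based forward and right vectors plus world up, while look input feeds pitch and yaw.
; Interact line-traces from the pawn's Head along the camera forward and calls I_Interactable on the hit actor.
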(event `self.ReceiveBeginPlay`
  (bind _returnvalue (subsystem `EnhancedInputLocalPlayerSubsystem`))
  ;[1 0.2865 0.8775] IMC
  (`/Engine/EditorBlueprintResources/StandardMacros.IsValid` _returnvalue
    (:`Is Valid`
      (`EnhancedInputSubsystemInterface.AddMappingContext` _returnvalue "/Game/A4GPContent/Inputs/IMC_MyDefaultIMC.IMC_MyDefaultIMC" 0 (struct))
      (bind _asbp_my_default_pawn (cast `/Game/A4GPContent/BP/BP_MyDefaultPawn` (`GameplayStatics.GetPlayerPawn` 0)))
      (set `self.MyDefaultPawn` _asbp_my_default_pawn))))

(event `self.ReceiveDestroyed`
  (bind _returnvalue (subsystem `EnhancedInputLocalPlayerSubsystem`))
  ;[1 0.2865 0.8775] IMC
  (`/Engine/EditorBlueprintResources/StandardMacros.IsValid` _returnvalue
    (:`Is Valid`
      (`EnhancedInputSubsystemInterface.RemoveMappingContext` _returnvalue "/Game/A4GPContent/Inputs/IMC_MyDefaultIMC.IMC_MyDefaultIMC" (struct)))))

(event `EnhancedInput|/Game/A4GPContent/Inputs/Actions/IA_MyPawnMove`
  (params (ActionValue :type "Vector Structure") (ElapsedSeconds :type "Float (double-precision)") (TriggeredSeconds :type "Float (double-precision)") (InputAction :type "InputAction Object Reference" :default "/Game/A4GPContent/Inputs/Actions/IA_MyPawnMove.IA_MyPawnMove"))
  (bind (_returnvalue_roll _returnvalue_pitch _returnvalue_yaw) (`KismetMathLibrary.BreakRotator` (`self.GetControlRotation`)))
  (bind _mydefaultpawn (`self.MyDefaultPawn`))
  ;[0.03559 0.5864 1] Movement
  (:`Triggered`
    (`/Engine/EditorBlueprintResources/StandardMacros.IsValid` _mydefaultpawn
      (:`Is Valid`
        ;;[1 1 1] Forward
        (`Pawn.AddMovementInput` _mydefaultpawn (`KismetMathLibrary.GetForwardVector` (`KismetMathLibrary.MakeRotator` _returnvalue_roll 0.0 _returnvalue_yaw)) ActionValue_X false)
        ;;[1 1 1] Lateral
        (`Pawn.AddMovementInput` _mydefaultpawn (`KismetMathLibrary.GetRightVector` (`KismetMathLibrary.MakeRotator` _returnvalue_roll 0.0 _returnvalue_yaw)) ActionValue_Y false)
        ;;[1 1 1] Vertical
        (`Pawn.AddMovementInput` _mydefaultpawn (0.0 0.0 1.0) ActionValue_Z false)))))

(event `EnhancedInput|/Game/A4GPContent/Inputs/Actions/IA_MyPawnLook`
  (params (ActionValue :type "Vector2D Structure") (ElapsedSeconds :type "Float (double-precision)") (TriggeredSeconds :type "Float (double-precision)") (InputAction :type "InputAction Object Reference" :default "/Game/A4GPContent/Inputs/Actions/IA_MyPawnLook.IA_MyPawnLook"))
  ;[1 0.8862 0.002916] Rotation
  (:`Triggered`
    (`self.AddPitchInput` ActionValue_Y)
    (`self.AddYawInput` ActionValue_X)))

(event `EnhancedInput|/Game/A4GPContent/Inputs/Actions/IA_MyInteract`
  (params (ActionValue :type Boolean) (ElapsedSeconds :type "Float (double-precision)") (TriggeredSeconds :type "Float (double-precision)") (InputAction :type "InputAction Object Reference" :default "/Game/A4GPContent/Inputs/Actions/IA_MyInteract.IA_MyInteract"))
  (bind _mydefaultpawn (`self.MyDefaultPawn`))
  (bind _head (`/Game/A4GPContent/BP/BP_MyDefaultPawn.Head` _mydefaultpawn))
  (bind _camera (`/Game/A4GPContent/BP/BP_MyDefaultPawn.Camera` _mydefaultpawn))
  (bind _returnvalue (`SceneComponent.K2_GetComponentLocation` _head))
  (:`Completed`
    ;[1 1 1] Line Trace
    (`/Engine/EditorBlueprintResources/StandardMacros.IsValid` _mydefaultpawn
      (:`Is Valid`
        (`/Engine/EditorBlueprintResources/StandardMacros.IsValid` _head
          (:`Is Valid`
            (`/Engine/EditorBlueprintResources/StandardMacros.IsValid` _camera
              (:`Is Valid`
                (bind _interactdistance (`/Game/A4GPContent/BP/BP_MyDefaultPawn.GetInteractDistance` _mydefaultpawn))
                (bind _outhit (`KismetSystemLibrary.LineTraceSingle` _returnvalue (+ _returnvalue (* (`SceneComponent.GetForwardVector` _camera) _interactdistance)) "TraceTypeQuery1"))
                ;[1 1 1] Interact
                (bind _asi_interactable (cast `/Game/A4GPContent/Datas/Interfaces/I_Interactable` (`.HitActor` (`GameplayStatics.BreakHitResult` _outhit))))
                (`/Game/A4GPContent/Datas/Interfaces/I_Interactable.Interact` _asi_interactable)))))))))

(fn `UserConstructionScript`)